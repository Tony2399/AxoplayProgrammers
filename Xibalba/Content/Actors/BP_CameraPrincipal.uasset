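; BP_CameraPrincipal is the main camera actor, which follows the player character from a fixed offset along the Y axis.
; Every Tick it moves to the player capsule's X and offset Y position while keeping its own Z, so it ignores vertical movement, with no smoothing or sweep.
; An earlier mesh-based version and a debug log remain in the graph but never run.
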(event EventTick
  (params (DeltaSeconds :type Float%20%28single-precision%29))
  (bind _returnvalue (Game|GetPlayerCharacter 0))
  (bind _returnvalue_2 (Actor|GetComponentbyClass _returnvalue "/Script/Engine.CapsuleComponent"))
  (bind _returnvalue_3 (Transformation|GetWorldLocation _returnvalue_2))
  (bind (_x _y) (Math|Vector|BreakVector _returnvalue_3))
  (Transformation|SetActorLocation (Math|Vector|MakeVector _x (- _y 1.01e+03) (.Z (Math|Vector|BreakVector (Transformation|GetActorLocation)))) false false))

(fn ConstructionScript)